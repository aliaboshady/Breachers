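; Game instance that manages multiplayer sessions through Advanced Sessions: create, find, cancel, join and destroy.
; Creation advertises server, map and mode names, opens the level as a listen server, then applies match settings to the game state after a one-second delay.
; Plant and Defuse stores settings on the warm-up state for the next game mode.
; Search results fill a supplied scroll box with session rows; destroying a session returns to MainMenu.
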(event Custom|CreateSession
  (params (LevelName :type Name) (MaxPlayers :type Integer) (GameModeRef :type String) (NextGameModeRef :type String) (ServerName :type String) (MapName :type String) (GameModeName :type String) (InfiniteTime :type Boolean) (InfiniteMoney :type Boolean) (InfiniteRounds :type Boolean) (RoundTime :type Integer) (RoundsNumber :type Integer))
  (|AdvancedSession (Utilities|Array|MakeArray (Class|AdvancedSessionsLibrary|MakeLiteralSessionPropertyString "ServerName" ServerName) (Class|AdvancedSessionsLibrary|MakeLiteralSessionPropertyString "MapName" MapName) (Class|AdvancedSessionsLibrary|MakeLiteralSessionPropertyString "GameModeName" GameModeName)) (Game|GetPlayerController 0) MaxPlayers 0 false true false true true false false false true
    (:then
      (Default|CallOnCreateSession))
    (:OnSuccess
      (Game|OpenLevel(byName) LevelName true (Utilities|String|ToString(Text) (Utilities|Text|FormatText "listen{GameModeRef}" GameModeRef)))
      (CallFunction|SetGameSettings GameModeName NextGameModeRef InfiniteTime InfiniteMoney InfiniteRounds RoundTime RoundsNumber))))

(event Custom|FindSession
  (params (FoundSessionsScrollBox :type Scroll%20Box%20Object%20Reference))
  (bind _results (|FindSessionsAdvanced (Game|GetPlayerController 0) 10 false "AllServers" 0 false false false)
    (:OnSuccess
      (Default|CallOnFoundSessionResults)
      (Variables|Default|SetFoundSessions _results)
      (CallFunction|PopulateFoundSessions FoundSessionsScrollBox))))

(event Custom|PopulateFoundSessions
  (params (FoundSessionsScrollBox :type Scroll%20Box%20Object%20Reference))
  (bind _foundsessions (Variables|Default|GetFoundSessions))
  (Widget|Panel|ClearChildren FoundSessionsScrollBox)
  (if (> (Utilities|Array|Length _foundsessions) 0)
    (bind _array_element (Utilities|Array|ForEachLoopwithBreak _foundsessions)
      (:LoopBody
        (bind _returnvalue (UserInterface|CreateWidget "/Game/_Main/UI/MainMenu/FindGame/W_SessionInfoRow.W_SessionInfoRow_C" (Game|GetPlayerController 0)))
        (Default|SetProperties _returnvalue _array_element)
        (Widget|Panel|AddChild FoundSessionsScrollBox _returnvalue)))))

(event Custom|StopFindingSessions
  (|CancelFindSessions (Game|GetPlayerController 0)))

(event Custom|JoinSession
  (params (Session :type Blueprint%20Session%20Result%20Structure))
  (if (Class|AdvancedSessionsLibrary|IsValidSession Session)
    (|JoinSession (Game|GetPlayerController 0) Session
      (:then
        (Default|CallOnJoinSession)))))

(event Custom|SetGameSettings
  (params (GameModeName :type String) (NextGameModeRef :type String) (InfiniteTime :type Boolean) (InfiniteMoney :type Boolean) (InfiniteRounds :type Boolean) (RoundTime :type Integer) (RoundsNumber :type Integer))
  (bind _returnvalue (Game|GetGameState))
  (Utilities|FlowControl|Delay 1.0)
  (switch string GameModeName
    (:Team%20DeathMatch
      (bind _asdeath_match_game_state (Utilities|Casting|CastToDeathMatchGameState _returnvalue :!label _label))
      (Variables|/Script/Breachers.DeathMatchGameState|SetbUnlimitedTime _asdeath_match_game_state InfiniteTime)
      (bind _asbreachers_game_state (Utilities|Casting|CastToBreachersGameState _returnvalue))
      (Variables|/Script/Breachers.BreachersGameState|SetCountDownTimeSpan _asbreachers_game_state (Math|Timespan|MakeTimespan 0 0 RoundTime 0 0)))
    (:Free%20For%20All
      (goto _label))
    (:Plant%20And%20Defuse
      (bind _aswarm_up_game_state (Utilities|Casting|CastToWarmUpGameState _returnvalue))
      (Class|WarmUpGameState|SetUnlimitedMoneyNextGM _aswarm_up_game_state InfiniteMoney)
      (Class|WarmUpGameState|SetUnlimitedRoundsNextGM _aswarm_up_game_state InfiniteRounds)
      (Class|WarmUpGameState|SetRoundTimeinMinutesNextGM _aswarm_up_game_state RoundTime)
      (Class|WarmUpGameState|SetRoundNumberPerHalfNextGM _aswarm_up_game_state RoundsNumber)
      (Class|WarmUpGameState|SetGameModeRefNextGM _aswarm_up_game_state NextGameModeRef))))

(event EventDestroyGameSession
  (|DestroySession (Game|GetPlayerController 0)
    (:then
      (Game|OpenLevel(byObjectReference) "/Game/_Main/Maps/MainMenu.MainMenu"))))