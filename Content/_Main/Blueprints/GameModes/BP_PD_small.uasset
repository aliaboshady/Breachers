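; BP_PD_small is a game mode Blueprint that configures match rules from the options string it is launched with.
; On BeginPlay, a sequence parses option keys for unlimited money, unlimited rounds, round time in minutes and rounds per half.
; The two flags switch on the parsed text to set booleans, while the round values convert to integers before reaching their setters.
; The graph contains no other gameplay logic.
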(event EventBeginPlay
  (bind _optionsstring (Variables|Default|GetOptionsString))
  (Utilities|FlowControl|Sequence
    (:then_0
      (switch string (Class|GameplayStatics|ParseOption _optionsstring "UnlimitedMoney")
        (:true
          (Class|PlantandDefuseGameMode|SetUnlimitedMoney true))
        (:false
          (Class|PlantandDefuseGameMode|SetUnlimitedMoney false))))
    (:then_1
      (switch string (Class|GameplayStatics|ParseOption _optionsstring "UnlimitedRounds")
        (:true
          (Class|PlantandDefuseGameMode|SetUnlimitedRounds true))
        (:false
          (Class|PlantandDefuseGameMode|SetUnlimitedRounds false))))
    (:then_2
      (Class|PlantandDefuseGameMode|SetRoundTime (Math|Conversions|ToInteger(Byte) (Class|GameplayStatics|ParseOption _optionsstring "RoundTimeInMinutes"))))
    (:then_3
      (Class|PlantandDefuseGameMode|SetRoundNumber (Math|Conversions|ToInteger(Byte) (Class|GameplayStatics|ParseOption _optionsstring "RoundNumberPerHalf"))))))

(fn ConstructionScript)